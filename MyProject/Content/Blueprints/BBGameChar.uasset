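; Side-moving Paper2D player character with jumping and accelerating movement along Y, clamped by YLimit.
; Forward and Backward axes ramp speed and set capsule location directly without sweep, only while grounded.
; Jump switches to the Idle flipbook; hitting an actor named "Floor" restores Juoksu and clears IsAirborne.
; Tick resets forward acceleration to default once a timed effect expires; nothing here starts that effect.
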(event OnComponentHit(CapsuleComponent)
  (params (HitComponent :type Primitive%20Component%20Object%20Reference) (OtherActor :type Actor%20Object%20Reference) (OtherComp :type Primitive%20Component%20Object%20Reference) (NormalImpulse :type Vector :default "0, 0, 0") (Hit :type Hit%20Result%20Structure%20%28by%20ref%29))
  ;[1 1 1] Hypyn lopetus
  (if (Utilities|Enum|Equal(Enum) (Utilities|GetObjectName OtherActor) "Floor")
    (Sprite|SetFlipbook (Variables|Default|GetSprite) "/Game/Flipbooks/juoksu.juoksu")
    (Variables|Default|SetisAirborne false)))

(event EventBeginPlay)

(event Collision|EventActorBeginOverlap
  (params (OtherActor :type Actor%20Object%20Reference)))

(event EventTick
  (params (DeltaSeconds :type Float%20%28single-precision%29))
  ;[1 1 1] Katsotaan joko efektin pitäisi loppua
  (if (> (- (Utilities|Time|GetGameTimeinSeconds) (Variables|Default|GetEffectStart)) (Variables|Default|GetEffectDuration))
    ;[1 1 1] Palautetaan alku nopeus
    (Variables|Default|Setacc (Variables|Default|Getdefaultacc))))

(event Input|ActionEvents|InputActionJump
  (params (Key :type Key%20Structure))
  ;[1 1 1] Hyppy
  (:Pressed
    (Character|Jump)
    (Sprite|SetFlipbook (Variables|Default|GetSprite) "/Game/Flipbooks/idle.idle")
    (Variables|Default|SetisAirborne true))
  (:Released
    (Character|StopJumping)))

(event Input|AxisEvents|InputAxisForward
  (params (AxisValue :type Float%20%28single-precision%29))
  (bind _capsulecomponent (Variables|Collision|GetCapsuleComponent))
  (bind _returnvalue (Transformation|GetWorldLocation _capsulecomponent))
  (bind (_x _y _z) (Math|Vector|BreakVector _returnvalue))
  ;[1 1 1] Eteenpäin liikkuminen
  (if (and (and (> AxisValue 0.0) (Math|Boolean|NotEqual(Boolean) (Variables|Default|GetisAirborne) true)) (< (.Y (Math|Vector|BreakVector (Transformation|GetWorldLocation (Variables|Collision|GetCapsuleComponent)))) (Variables|Default|GetyLimit)))
    (Variables|Default|SetySpeed (+ (Variables|Default|GetySpeed) (Variables|Default|Getacc)))
    (Transformation|SetWorldLocation _capsulecomponent (Math|Vector|MakeVector _x (+ _y (Variables|Default|GetySpeed)) _z) false false)
    (else
      (Variables|Default|SetySpeed 3.0)
      (Variables|Default|SetDirectionNotChanged true))))

(event Input|AxisEvents|InputAxisBackward
  (params (AxisValue :type Float%20%28single-precision%29))
  (bind _capsulecomponent (Variables|Collision|GetCapsuleComponent))
  (bind _returnvalue (Transformation|GetWorldLocation _capsulecomponent))
  (bind (_x _y _z) (Math|Vector|BreakVector _returnvalue))
  ;[1 1 1] Taaksepäin liikkuminen
  (if (Math|Boolean|ANDBoolean (> AxisValue 0.0) (> (.Y (Math|Vector|BreakVector (Transformation|GetWorldLocation (Variables|Collision|GetCapsuleComponent)))) (- 0.0 (Variables|Default|GetyLimit))) (not (Variables|Default|GetisAirborne)))
    (Variables|Default|SetbackwardAcceleration (+ (Variables|Default|GetbackwardAcceleration) 0.1))
    (Transformation|SetWorldLocation (Variables|Collision|GetCapsuleComponent) (Math|Vector|MakeVector _x (- _y (Variables|Default|GetbackwardAcceleration)) _z) false false)
    (else
      (Variables|Default|SetbackwardAcceleration 0.0)
      (Variables|Default|SetDirectionNotChanged true))))

(fn ConstructionScript)