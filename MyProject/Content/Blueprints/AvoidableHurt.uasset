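; AvoidableHurt is a hazard Blueprint that hurts a character by draining its LifeForce when ApplyEffect is called.
; The damage is the Damage value scaled by elapsed game time, so hits grow harsher the longer the game runs.
; LifeForce is clamped at zero, and each hit also sets the hazard's own Speed to a fixed value.
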(event EventBeginPlay
  (|CallParentFunction) ; This node is disabled and will not be called.\nDrag off pins to build functionality.
)

(event Collision|EventActorBeginOverlap
  (params (OtherActor :type Actor%20Object%20Reference)))

(event EventTick
  (params (DeltaSeconds :type Float%20%28single-precision%29)))

(event EventApplyEffect
  (params (Charachter :type BB%20Game%20Char%20Object%20Reference))
  ;[1 1 1] Katsotaan meneekö elämä mioinukselle ja tehdään sen mukaan vähennystä elämästä
  (if (> (- (Variables|/Game/Blueprints/BBGameChar.BBGameChar_C|GetLifeForce Charachter) (* (/ (Utilities|Time|GetGameTimeinSeconds) 1e+01) (Variables|Default|GetDamage))) 0.0)
    (Variables|/Game/Blueprints/BBGameChar.BBGameChar_C|SetLifeForce Charachter (- (Variables|/Game/Blueprints/BBGameChar.BBGameChar_C|GetLifeForce Charachter) (* (/ (Utilities|Time|GetGameTimeinSeconds) 1e+01) (Variables|Default|GetDamage))))
    (else
      (Variables|/Game/Blueprints/BBGameChar.BBGameChar_C|SetLifeForce Charachter 0.0)))
  (Variables|Default|SetSpeed 5e+02))

(fn ConstructionScript
  (|CallParentFunction))