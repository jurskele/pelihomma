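; AvoidableSlow is an avoidable hazard that slows the player when its ApplyEffect event runs.
; ApplyEffect stores the character and plays a paint splat sound at the world origin.
; If the character's default speed minus SpeedDrain stays above a small minimum, it sets a very low Acc on the player, stamps EffectStart with game time for the effect's duration, and sets its own Speed.
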(event EventBeginPlay
  (|CallParentFunction) ; This node is disabled and will not be called.\nDrag off pins to build functionality.
)

(event Collision|EventActorBeginOverlap
  (params (OtherActor :type Actor%20Object%20Reference)))

(event EventTick
  (params (DeltaSeconds :type Float%20%28single-precision%29)))

(event EventApplyEffect
  (params (Charachter :type BB%20Game%20Char%20Object%20Reference))
  ;[1 1 1] Vähennetään pelaajan vauhtia
  (Variables|Default|Setplayer Charachter)
  (Audio|PlaySoundatLocation "/Game/Sounds/large_paint_splat.large_paint_splat" "0, 0, 0" "0, 0, 0" 0.4 1.0 0.0 0 0 0)
  (if (> (- (Variables|/Game/Blueprints/BBGameChar.BBGameChar_C|GetDefaultSpeed Charachter) (Variables|Default|GetspeedDrain)) 1.0)
    (Variables|/Game/Blueprints/BBGameChar.BBGameChar_C|Setacc (Variables|Default|Getplayer) 0.01)
    ;[1 1 1] sijoitetaan pelin aika efektin kestoa varten
    (Variables|/Game/Blueprints/BBGameChar.BBGameChar_C|SetEffectStart (Variables|Default|Getplayer) (Utilities|Time|GetGameTimeinSeconds))
    (Variables|Default|SetSpeed 5e+02)))

(fn ConstructionScript
  (|CallParentFunction))