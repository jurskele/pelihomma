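; CollectiblesPool is an object pool that spawns and recycles Collectibles scrolling along negative Y.
; CreateCollectible spawns items at the start Y with random height and a time-influenced speed, adding them to ThePool until MaxCollectibles is reached.
; UpdateCollectible moves each pooled item by its Speed per call, wrapping those past the far edge back to the start with new height and speed.
; Its own events are empty, leaving both functions to external callers.
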(event EventBeginPlay)

(event Collision|EventActorBeginOverlap
  (params (OtherActor :type Actor%20Object%20Reference)))

(event EventTick
  (params (DeltaSeconds :type Float%20%28single-precision%29)))

(fn ConstructionScript)

(fn CreateCollectible
  ;[1 1 1] Tarkistetaan ettei kerättäviä ole liikaa
  (if (< (Variables|Default|GetnrOfCollectibles) (Variables|Default|GetmaxCollectibles))
    ;[1 1 1] Luodaan kerättävä tavara
    (bind _returnvalue (Game|SpawnActorfromClass "/Game/Blueprints/Collectibles.Collectibles_C" (Math|Transform|MakeTransform (Math|Vector|MakeVector 0.0 (Variables|Default|GetcollectibleStartY) (Math|Random|RandomFloatinRange 5e+01 8e+02)) "0,90.000000, 0") "Undefined" 0 0))
    (Variables|/Game/Blueprints/Collectibles.Collectibles_C|SetSpeed _returnvalue (Math|Random|RandomFloatinRange (/ (/ (Utilities|Time|GetGameTimeinSeconds) 4.0) (Variables|/Game/Blueprints/Collectibles.Collectibles_C|GetSpeed _returnvalue)) (Variables|/Game/Blueprints/Collectibles.Collectibles_C|GetSpeed _returnvalue)))
    ;[1 1 1] Lisätään luotu kerättävä esine "altaaseen" ja nostetaan laskuria
    (Utilities|Array|Insert (Variables|Default|GetthePool) _returnvalue (Variables|Default|GetnrOfCollectibles))
    (Math|Integer|IncrementInt (Variables|Default|GetnrOfCollectibles))))

(fn UpdateCollectible
  ;[1 1 1] Päivitetään kerättävät asiat
  (for (_array_element _array_index) (Variables|Default|GetthePool)
    ;[1 1 1] Tarkistetaan onko kerättävä esine jo tarpeeksi vasemmalla
    (LocalVariables|SetarrayElement _array_element)
    (LocalVariables|SetarrayIndex _array_index)
    (if (< (.Y (Math|Vector|BreakVector (Transformation|GetWorldLocation (Variables|/Script/Engine.Actor|GetRootComponent _array_element)))) (- 0.0 (Variables|Default|GetcollectibleStartY)))
      ;[1 1 1] Siirretään esine ruudun alkuun ja muokataan sijainti ja vauhti
      (Transformation|SetWorldLocation (Variables|/Script/Engine.Actor|GetRootComponent (LocalVariables|GetarrayElement)) (Math|Vector|MakeVector 0.0 (Variables|Default|GetcollectibleStartY) (Math|Random|RandomFloatinRange 5e+01 8e+02)) false false)
      (bind _ascollectibles (Utilities|Casting|CastToCollectibles (LocalVariables|GetarrayElement)))
      (Variables|/Game/Blueprints/Collectibles.Collectibles_C|SetSpeed _ascollectibles (Math|Random|RandomFloatinRange 7.0 15.0))
      (else
        ;[1 1 1] Jos ei liian vasemmalla liikutetaan esinettä
        (bind _ascollectibles_2 (Utilities|Casting|CastToCollectibles _array_element))
        (Transformation|AddWorldOffset (Variables|/Script/Engine.Actor|GetRootComponent _array_element) (Math|Vector|MakeVector 0.0 (- 0.0 (Variables|/Game/Blueprints/Collectibles.Collectibles_C|GetSpeed _ascollectibles_2)) 0.0) false false)))))