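; Object pool of obstacles to avoid that scroll along negative Y across the playfield.
; CreateAvoidable spawns a random class at the start edge and a random height until the cap is reached, with a randomized speed whose range depends on game time.
; UpdateAvoidable moves each pooled obstacle by its speed per call, recycling those past the opposite edge with new height and speed.
; Both functions rely on outside callers.
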(event EventBeginPlay)

(event Collision|EventActorBeginOverlap
  (params (OtherActor :type Actor%20Object%20Reference)))

(event EventTick
  (params (DeltaSeconds :type Float%20%28single-precision%29)))

(fn ConstructionScript)

(fn CreateAvoidable
  (bind _avoidables (Variables|Default|GetAvoidables))
  ;[1 1 1] Tarkistetaan ettei kerättäviä ole liikaa
  (if (< (Variables|Default|GetnrOfAvoidables) (Variables|Default|GetmaxAvoidables))
    ;[1 1 1] Luodaan kerättävä tavara
    (bind _returnvalue (Game|SpawnActorfromClass (Utilities|Array|Get(acopy) _avoidables (Math|Random|RandomIntegerinRange 0 (Utilities|Array|LastIndex _avoidables))) (Math|Transform|MakeTransform (Math|Vector|MakeVector 0.0 (Variables|Default|GetavoidableStartY) (Math|Random|RandomFloatinRange 5e+01 8e+02)) "0,90.000000, 0") "Undefined" 0 0))
    (bind _asavoidables (Utilities|Casting|CastToAvoidables _returnvalue))
    (Variables|/Game/Blueprints/Avoidables.Avoidables_C|SetSpeed _asavoidables (Math|Random|RandomFloatinRange (/ (/ (Utilities|Time|GetGameTimeinSeconds) 4.0) (Variables|/Game/Blueprints/Avoidables.Avoidables_C|GetSpeed _asavoidables)) (Variables|/Game/Blueprints/Avoidables.Avoidables_C|GetSpeed _asavoidables)))
    ;[1 1 1] Lisätään luotu kerättävä esine "altaaseen" ja nostetaan laskuria
    (Utilities|Array|Insert (Variables|Default|GetthePool) _asavoidables (Variables|Default|GetnrOfAvoidables))
    (Math|Integer|IncrementInt (Variables|Default|GetnrOfAvoidables))))

(fn UpdateAvoidable
  ;[1 1 1] Päivitetään väistettävät asiat
  (for _array_element (Variables|Default|GetthePool)
    ;[1 1 1] Tarkistetaan onko väistettävä esine jo tarpeeksi vasemmalla
    (LocalVariables|SetarrayElement _array_element)
    (if (< (.Y (Math|Vector|BreakVector (Transformation|GetWorldLocation (Variables|/Script/Engine.Actor|GetRootComponent _array_element)))) (- 0.0 (Variables|Default|GetavoidableStartY)))
      ;[1 1 1] Siirretään esine ruudun alkuun ja muokataan sijainti ja vauhti
      (Transformation|SetWorldLocation (Variables|/Script/Engine.Actor|GetRootComponent (LocalVariables|GetarrayElement)) (Math|Vector|MakeVector 0.0 (Variables|Default|GetavoidableStartY) (Math|Random|RandomFloatinRange 5e+01 8e+02)) false false)
      (bind _asavoidables (Utilities|Casting|CastToAvoidables (LocalVariables|GetarrayElement)))
      (Variables|/Game/Blueprints/Avoidables.Avoidables_C|SetSpeed _asavoidables (Math|Random|RandomFloatinRange 7.0 15.0))
      (else
        ;[1 1 1] Jos ei liian vasemmalla liikutetaan esinettä
        (bind _asavoidables_2 (Utilities|Casting|CastToAvoidables _array_element))
        (Transformation|AddWorldOffset (Variables|/Script/Engine.Actor|GetRootComponent _array_element) (Math|Vector|MakeVector 0.0 (- 0.0 (Variables|/Game/Blueprints/Avoidables.Avoidables_C|GetSpeed _asavoidables_2)) 0.0) false false)))))