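; RewardsPool manages a capped pool of collectible RewardCoins that scroll sideways along the Y axis.
; CreateReward spawns a coin at the start edge with random height and a randomized, time-influenced speed, then stores it until MaxRewards is reached.
; UpdateReward moves each coin by its Speed per call, recycling those past the opposite edge with new height and speed instead of destroying them.
; Its event graph is inactive, so neither function is called here.
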(event EventBeginPlay)

(event Collision|EventActorBeginOverlap
  (params (OtherActor :type Actor%20Object%20Reference)))

(event EventTick
  (params (DeltaSeconds :type Float%20%28single-precision%29)))

(fn ConstructionScript)

(fn CreateReward
  ;[1 1 1] Tarkistetaan ettei palkintoja ole liikaa
  (if (< (Variables|Default|GetnrOfRewards) (Variables|Default|GetmaxRewards))
    ;[1 1 1] Luodaan kerättävä palkinto
    (bind _returnvalue (Game|SpawnActorfromClass "/Game/Blueprints/RewardCoins.RewardCoins_C" (Math|Transform|MakeTransform (Math|Vector|MakeVector 0.0 (Variables|Default|GetRewardsStartY) (Math|Random|RandomFloatinRange 5e+01 8e+02)) "0,90.000000, 0") "Undefined" 0 0))
    (Variables|/Game/Blueprints/RewardCoins.RewardCoins_C|SetSpeed _returnvalue (Math|Random|RandomFloatinRange (/ (/ (Utilities|Time|GetGameTimeinSeconds) 4.0) (Variables|/Game/Blueprints/RewardCoins.RewardCoins_C|GetSpeed _returnvalue)) (Variables|/Game/Blueprints/RewardCoins.RewardCoins_C|GetSpeed _returnvalue)))
    ;[1 1 1] Lisätään luotu kerättävä esine "altaaseen" ja nostetaan laskuria
    (Utilities|Array|Insert (Variables|Default|GetthePool) _returnvalue (Variables|Default|GetnrOfRewards))
    (Math|Integer|IncrementInt (Variables|Default|GetnrOfRewards))))

(fn UpdateReward
  ;[1 1 1] Päivitetään kerättävät asiat
  (for (_array_element _array_index) (Variables|Default|GetthePool)
    ;[1 1 1] Tarkistetaan onko kerättävä esine jo tarpeeksi vasemmalla
    (LocalVariables|SetarrayElement _array_element)
    (LocalVariables|SetarrayIndex _array_index)
    (if (< (.Y (Math|Vector|BreakVector (Transformation|GetWorldLocation (Variables|/Script/Engine.Actor|GetRootComponent _array_element)))) (- 0.0 (Variables|Default|GetRewardsStartY)))
      ;[1 1 1] Siirretään esine ruudun alkuun ja muokataan sijainti ja vauhti
      (Transformation|SetWorldLocation (Variables|/Script/Engine.Actor|GetRootComponent (LocalVariables|GetarrayElement)) (Math|Vector|MakeVector 0.0 (Variables|Default|GetRewardsStartY) (Math|Random|RandomFloatinRange 5e+01 8e+02)) false false)
      (bind _asreward_coins (Utilities|Casting|CastToRewardCoins (LocalVariables|GetarrayElement)))
      (Variables|/Game/Blueprints/RewardCoins.RewardCoins_C|SetSpeed _asreward_coins (Math|Random|RandomFloatinRange 7.0 15.0))
      (else
        ;[1 1 1] Jos ei liian vasemmalla liikutetaan esinettä
        (bind _asreward_coins_2 (Utilities|Casting|CastToRewardCoins _array_element))
        (Transformation|AddWorldOffset (Variables|/Script/Engine.Actor|GetRootComponent _array_element) (Math|Vector|MakeVector 0.0 (- 0.0 (Variables|/Game/Blueprints/RewardCoins.RewardCoins_C|GetSpeed _asreward_coins_2)) 0.0) false false)))))