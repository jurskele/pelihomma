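; Collectible actor that restores the BBGameChar player's LifeForce when it overlaps the collectible's Box component.
; The overlap checks the actor's display name and casts it, then, if health is below full, adds Effect scaled by elapsed game time, capped at full.
; After applying the boost it sets its own Speed variable to a fixed value; the file shows no destroy step.
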(event OnComponentBeginOverlap(Box)
  (params (OverlappedComponent :type Primitive%20Component%20Object%20Reference) (OtherActor :type Actor%20Object%20Reference) (OtherComp :type Primitive%20Component%20Object%20Reference) (OtherBodyIndex :type Integer) (bFromSweep :type Boolean) (SweepResult :type Hit%20Result%20Structure%20%28by%20ref%29))
  (if (Utilities|Enum|Equal(Enum) (Utilities|GetDisplayName OtherActor) "BBGameChar")
    (bind _asbbgame_char (Utilities|Casting|CastToBBGameChar OtherActor))
    ;[1 1 1] Tarkistetaan onko pelaajan elämäpisteet jo maksimissa
    (if (< (Variables|/Game/Blueprints/BBGameChar.BBGameChar_C|GetLifeForce _asbbgame_char) 1.0)
      ;[1 1 1] Tarkastetaan onko boostattu summa enemmän kuin maksimi elämämäärä
      (if (<= (+ (Variables|/Game/Blueprints/BBGameChar.BBGameChar_C|GetLifeForce _asbbgame_char) (* (/ (Utilities|Time|GetGameTimeinSeconds) 5.0) (Variables|Default|Geteffect))) 1.0)
        (Variables|/Game/Blueprints/BBGameChar.BBGameChar_C|SetLifeForce _asbbgame_char (+ (Variables|/Game/Blueprints/BBGameChar.BBGameChar_C|GetLifeForce _asbbgame_char) (* (/ (Utilities|Time|GetGameTimeinSeconds) 5.0) (Variables|Default|Geteffect))))
        (else
          (Variables|/Game/Blueprints/BBGameChar.BBGameChar_C|SetLifeForce _asbbgame_char 1.0)))
      (Variables|Default|SetSpeed 5e+02))))

(event EventBeginPlay)

(event Collision|EventActorBeginOverlap
  (params (OtherActor :type Actor%20Object%20Reference)))

(event EventTick
  (params (DeltaSeconds :type Float%20%28single-precision%29)))

(fn ConstructionScript)